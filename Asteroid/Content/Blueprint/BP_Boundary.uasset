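; BP_Boundary is a box-triggered boundary that shifts whatever overlaps it by a configurable MoveX/MoveY offset, apparently for screen wrapping.
; For BP_Asteroid, it moves the root component, first adjusting each offset against its sign by an amount scaled to asteroid size (zero counts as positive).
; Other actors have their overlapping component moved by the raw offset.
; The Mover macro applies the relative shift through a zero-duration MoveComponentTo.
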(event `self.Box.OnComponentBeginOverlap`
  (params (OverlappedComponent :type "PrimitiveComponent Object Reference") (OtherActor :type "Actor Object Reference") (OtherComp :type "PrimitiveComponent Object Reference") (OtherBodyIndex :type Integer) (bFromSweep :type Boolean) (SweepResult :type "HitResult Structure (by ref)"))
  (bind _asbp_asteroid (cast `/Game/Blueprint/BP_Asteroid` OtherActor)
    (:`then`
      (bind _componente_raiz (`/Game/Blueprint/BP_Asteroid.Get_Componente_Raiz` _asbp_asteroid))
      (bind _tamanho (`/Game/Blueprint/BP_Asteroid.Get_Tamanho` _asbp_asteroid))
      (bind _returnvalue (`self.Asteroid_Sise_Considerator` (`self.MoveY`) _tamanho))
      (bind _returnvalue_2 (`self.Asteroid_Sise_Considerator` (`self.MoveX`) _tamanho))
      (`self.Mover` _componente_raiz _returnvalue_2 _returnvalue))
    (:`CastFailed`
      (`self.Mover` OtherComp (`self.MoveX`) (`self.MoveY`)))))

(fn `Asteroid_Sise_Considerator`
  (params (InputPin :type Integer) (Tamanho :type Integer))
  (returns (ReturnValue :type Integer))
  (bind _returnvalue (* Tamanho 200))
  (if (< InputPin 0)
    (return (+ InputPin _returnvalue))
    (else
      (return (- InputPin _returnvalue)))))

(fn `UserConstructionScript`)