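; Player ship character for an Asteroids-style shooter, handling thrust, yaw rotation, shooting and a random Shift teleport, noted as breaking bullet collision.
; BeginPlay creates the score widget, refreshed by SetScore, and switches view to the level's first CameraActor.
; Tick also drives asteroid spawning at random arena points with random speeds.
; Delay-based cooldown flags throttle both asteroids and bullets, which launch along the ship's forward vector with it recorded as origin.
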(event `InputAxis|Q_Listener`
  (params (AxisValue :type "Float (single-precision)")))

(event `Set Score`
  (`/Game/UI/Widgets/W_Score.Update_Score` (`self.Score_Board`) (`KismetTextLibrary.Conv_IntToText` (`self.Score`)) ""))

(event `InputAxis|E_Listener`
  (params (AxisValue :type "Float (single-precision)")))

(event `self.ReceiveBeginPlay`
  ;[1 1 1] Configura a câmera
  (bind _returnvalue (`|CreateWidget` "/Game/UI/Widgets/W_Score.W_Score_C" (`self.GetLocalViewingPlayerController` self)))
  (bind _output_get (set `self.Score_Board` _returnvalue))
  (`UserWidget.AddToViewport` _output_get 0)
  (bind _outactors (`GameplayStatics.GetAllActorsOfClass` "/Script/Engine.CameraActor"))
  (`PlayerController.SetViewTargetWithBlend` (`self.GetLocalViewingPlayerController`) (`|GetArrayItem` _outactors) 0.0 "VTBlend_Linear" 0.0 false))

(event `InputAxis|Acelerate`
  (params (AxisValue :type "Float (single-precision)"))
  ;[1 1 1] Responssável pela aceleração
  (`self.AddMovementInput` (`self.GetActorForwardVector`) AxisValue))

(event `InputAxis|Disparar`
  (params (AxisValue :type "Float (single-precision)"))
  ;[1 1 1] Responsável por disparar
  (`/Engine/EditorBlueprintResources/StandardMacros.CompareInt` (`KismetMathLibrary.FTrunc` AxisValue) 1
    (:`==`
      (`self.Bullet_Spawner`)
      (`self.Cooldown_Shoot` (`self.Shoot_CD_Time`)))))

(event `InputAxis|SpinRight`
  (params (AxisValue :type "Float (single-precision)"))
  ;[1 1 1] responssável por girar a nave
  (`self.K2_AddActorLocalRotation` (`KismetMathLibrary.MakeRotator` 0.0 0.0 (* AxisValue (`KismetMathLibrary.Conv_IntToDouble` (`self.Rotation`))))))

(event `InputAxis|Teleporte`
  (params (AxisValue :type "Float (single-precision)"))
  ;[1 1 1] Tentativa de fazer a nave teleporta ao pressionar Shift, porém após o teleporte os seus disparos não apresentam colizor
  (`/Engine/EditorBlueprintResources/StandardMacros.CompareInt` (`KismetMathLibrary.FTrunc` AxisValue) 1
    (:`==`
      (`self.K2_SetActorRelativeTransform` self (`KismetMathLibrary.Conv_VectorToTransform` (+ (`SceneComponent.RelativeLocation` (`self.CapsuleComponent`)) (`KismetMathLibrary.MakeVector` (`KismetMathLibrary.Conv_IntToDouble` (`KismetMathLibrary.RandomIntegerInRange` -5500 5500)) (`KismetMathLibrary.Conv_IntToDouble` (`KismetMathLibrary.RandomIntegerInRange` -3500 3500)) 120.0))) false false))))

(event `self.ReceiveTick`
  (params (DeltaSeconds :type "Float (single-precision)"))
  ;[1 1 1] Responssável por spawnar os asteroides
  (if (not (`self.Asteroid_Cooldown`))
    (`self.Asteroid_Spawner`)
    (`self.Cooldown_Ateroid` (`self.Asteroid_CD_Time`))))

(fn `Get_Score`
  (returns (Score :type Integer))
  (return (`self.Score`)))

(fn `Sofre_Dano`)

(fn `UserConstructionScript`)