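; PC_Lobby is the lobby player controller, which shows the lobby UI and handles leaving the session.
; On BeginPlay it creates the W_Lobby widget, adds it to the viewport and sets Game and UI input focused on it.
; The Voltar (back) event destroys the current session and, on its then output, opens the Menu level.
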(event `Menu_Render`
  (bind _returnvalue (`|CreateWidget` "/Game/UI/Widgets/W_Lobby.W_Lobby_C" self))
  (`UserWidget.AddToViewport` _returnvalue 0)
  (`WidgetBlueprintLibrary.SetInputMode_GameAndUIEx` self _returnvalue))

(event `self.ReceiveBeginPlay`
  (`self.Menu_Render`))

(event `Voltar`
  (`DestroySessionCallbackProxy.DestroySession` self
    (:`then`
      (`GameplayStatics.OpenLevel` "Menu"))))

(fn `UserConstructionScript`)